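; Fabric1 module Blueprint for the mine base, a child that supplies the animations and work response for this module type.
; On BeginPlay it binds handlers to idle-animation, work-animation and work dispatchers, which are not fired in this graph.
; The animation handlers loop the idle or work animation on the Fabric1 mesh, while the work handler only prints a debug string.
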(event `self.ReceiveBeginPlay`
  (add `self.on_play_iddle_anim` (delegate `on_play_iddle_anim_Event_0`))
  (add `self.on_play_work_anim` (delegate `on_play_work_anim_Event_0`))
  (add `self.on_work` (delegate `on_work_Event`)))

(event `on_play_work_anim_Event_0`
  (`SkeletalMeshComponent.PlayAnimation` (`self.fabric1`) "/Game/GameObjects/MineBase/Modules/Fabric1/fabric1_work.fabric1_work" true))

(event `on_work_Event`
  (`KismetSystemLibrary.PrintString` "fabric1 work"))

(event `on_play_iddle_anim_Event_0`
  (`SkeletalMeshComponent.PlayAnimation` (`self.fabric1`) "/Game/GameObjects/MineBase/Modules/Fabric1/fabric1_iddle.fabric1_iddle" true))

(fn `UserConstructionScript`
  (`parent.UserConstructionScript`))