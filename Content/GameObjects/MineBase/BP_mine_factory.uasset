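; Mine factory base actor that spawns miner ships and serves as their docking point.
; On BeginPlay it sets its Luner data as a Factory, starts the module's idle animation, creates an info widget showing name and code, then spawns two miners in staggered order.
; Each miner appears at SpawnPoint and, after a short delay, is commanded to mine the assigned resource for this factory, both referenced by world code.
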(event `self.ReceiveBeginPlay`
  (bind (_cargosize _shieldsize _hullsize _team _friendenimy) (break `LunerData` (`self.lunerData`)))
  (set `self.lunerData` (make `LunerData` _cargosize _shieldsize _hullsize _team _friendenimy "Factory"))
  (bind _asbp_fabric_1_module (cast `/Game/GameObjects/MineBase/Modules/Fabric1/BP_fabric1_module` (`ChildActorComponent.ChildActor` (`self.BP_fabric1_module`))))
  (`/Game/GameObjects/MineBase/BP_base_module.on_play_iddle_anim` _asbp_fabric_1_module)
  (`self.Init` "MineFactory")
  (`self.on_create_info_widget`)
  (`KismetSystemLibrary.Delay` 1.0)
  (`self.spawn_ship`)
  (`KismetSystemLibrary.Delay` 1.0)
  (`self.spawn_ship`))

(event `spawn_ship`
  ;[1 1 1] test spawn miners
  (bind _returnvalue (`|SpawnActorFromClass` "/Game/GameObjects/MineShip/BP_miner_ship.BP_miner_ship_C" (`KismetMathLibrary.MakeTransform` (`SceneComponent.K2_GetComponentLocation` (`self.spawn_point`))) "Undefined" "OverrideRootScale" null null null null))
  (`KismetSystemLibrary.Delay` 1.0)
  (bind _asx_base_luner (cast `xBaseLuner` (`self.resource_actor`)))
  (`/Game/GameObjects/MineShip/BP_miner_ship.on_cmd_mine` _returnvalue (`xBaseLuner.worldCode` _asx_base_luner) (`self.worldCode`)))

(event `on_create_info_widget`
  (bind _returnvalue (`|CreateWidget` "/Game/GameObjects/MineBase/W_mine_factory_info.W_mine_factory_info_C" (`GameplayStatics.GetPlayerController` 0)))
  (bind _output_get (set `self.infoWidget` _returnvalue))
  (bind _asw_mine_factory_info (cast `/Game/GameObjects/MineBase/W_mine_factory_info` _output_get))
  (`TextBlock.SetText` (`/Game/GameObjects/MineBase/W_mine_factory_info.title` _asw_mine_factory_info) (`KismetTextLibrary.Conv_StringToText` (`self.lunerName`)))
  (`TextBlock.SetText` (`/Game/GameObjects/MineBase/W_mine_factory_info.Code` _asw_mine_factory_info) (`KismetTextLibrary.Conv_StringToText` (`self.worldCode`))))

(fn `getDockingLocation`
  (returns (ReturnValue :type "Vector Structure"))
  (return (`SceneComponent.K2_GetComponentLocation` (`self.spawn_point`))))

(fn `UserConstructionScript`)