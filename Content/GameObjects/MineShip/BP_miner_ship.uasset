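; Miner ship unit that takes stop, move and mine commands and passes them to its AI controller's blackboard.
; Mining and target-assignment events look up base and resource actors in the game mode's SpaceMap and store them as targets.
; Move resets the command to stop before writing the destination and setting move.
; An info widget shows name and world code, with its state updated through the command-action dispatcher.
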(event `on_cmd_action_Event_0` :!signature `self.on_cmd_action`
  (params (cmd :type String))
  ;[1 1 1] Info widjet actions
  (switch `string` cmd
    (:`stop`
      (bind _asw_miner_ship_info (cast `/Game/GameObjects/MineShip/W_miner_ship_info` (`self.infoWidget`)))
      (`/Game/GameObjects/MineShip/W_miner_ship_info.set_is_stop` _asw_miner_ship_info))
    (:`mine`
      (bind _asw_miner_ship_info_2 (cast `/Game/GameObjects/MineShip/W_miner_ship_info` (`self.infoWidget`)))
      (`/Game/GameObjects/MineShip/W_miner_ship_info.set_is_mine` _asw_miner_ship_info_2))
    (:`move`
      (bind _asw_miner_ship_info_3 (cast `/Game/GameObjects/MineShip/W_miner_ship_info` (`self.infoWidget`)))
      (`/Game/GameObjects/MineShip/W_miner_ship_info.set_is_move` _asw_miner_ship_info_3))))

(event `self.ReceiveBeginPlay`
  (`parent.ReceiveBeginPlay`)
  (`self.Init` "xMInerShip")
  (`self.on_create_info_widget`)
  (bind _asai_ctrl_miner (cast `/Game/GameObjects/MineShip/AI_ctrl_miner` (`self.GetController`)))
  (set `self.AICtrl` _asai_ctrl_miner)
  ;[1 1 1] on set base
  (add `self.on_set_base_target` (delegate `CustomEvent_0`))
  ;[1 1 1] on set resource
  (add `self.on_set_resource_target` (delegate `CustomEvent_1`))
  ;[1 1 1] Info widjet actions
  (add `self.on_cmd_action` (delegate `on_cmd_action_Event_0`)))

(event `CustomEvent_1` :!signature `self.on_set_resource_target`
  (params (targetActor :type String))
  ;[1 1 1] on set resource
  (bind _asxspace_game_mode (cast `xspaceGameMode` (`GameplayStatics.GetGameMode`)))
  (bind (_value _returnvalue) (`BlueprintMapLibrary.Map_Find` (`SpaceWorld.spaceMap` (`xspaceGameMode.xSpaceWorld` _asxspace_game_mode)) targetActor))
  (if _returnvalue
    (bind _asx_base_luner (cast `xBaseLuner` _value))
    (set `self.resource_target` _asx_base_luner)))

(event `CustomEvent_0` :!signature `self.on_set_base_target`
  (params (targetActor :type String))
  ;[1 1 1] on set base
  (bind _asxspace_game_mode (cast `xspaceGameMode` (`GameplayStatics.GetGameMode`)))
  (bind (_value _returnvalue) (`BlueprintMapLibrary.Map_Find` (`SpaceWorld.spaceMap` (`xspaceGameMode.xSpaceWorld` _asxspace_game_mode)) targetActor))
  (if _returnvalue
    (bind _asx_base_luner (cast `xBaseLuner` _value))
    (set `self.base_target` _asx_base_luner)))

(event `on_create_info_widget`
  ;[1 1 1] Create info widget
  (bind _returnvalue (`|CreateWidget` "/Game/GameObjects/MineShip/W_miner_ship_info.W_miner_ship_info_C" (`GameplayStatics.GetPlayerController` 0)))
  (bind _output_get (set `self.infoWidget` _returnvalue))
  (bind _asw_miner_ship_info (cast `/Game/GameObjects/MineShip/W_miner_ship_info` _output_get))
  (`/Game/GameObjects/MineShip/W_miner_ship_info.set_is_stop` _asw_miner_ship_info)
  (`TextBlock.SetText` (`/Game/GameObjects/MineShip/W_miner_ship_info.title` _asw_miner_ship_info) (`KismetTextLibrary.Conv_StringToText` (`self.lunerName`)))
  (`TextBlock.SetText` (`/Game/GameObjects/MineShip/W_miner_ship_info.Code` _asw_miner_ship_info) (`KismetTextLibrary.Conv_StringToText` (`self.worldCode`))))

(event `on_cmd_mine`
  (params (mine_resource :type String) (factory :type String))
  ;[1 1 1] cmd mine
  (bind _asxspace_game_mode (cast `xspaceGameMode` (`GameplayStatics.GetGameMode`)))
  (bind (_value _returnvalue) (`BlueprintMapLibrary.Map_Find` (`SpaceWorld.spaceMap` (`xspaceGameMode.xSpaceWorld` _asxspace_game_mode)) factory))
  (if _returnvalue
    (bind _asx_base_luner (cast `xBaseLuner` _value))
    (set `self.base_target` _asx_base_luner)
    (bind _asxspace_game_mode_2 (cast `xspaceGameMode` (`GameplayStatics.GetGameMode`)))
    (bind (_value_2 _returnvalue_2) (`BlueprintMapLibrary.Map_Find` (`SpaceWorld.spaceMap` (`xspaceGameMode.xSpaceWorld` _asxspace_game_mode_2)) mine_resource))
    (if _returnvalue_2
      (bind _asx_base_luner_2 (cast `xBaseLuner` _value_2))
      (set `self.resource_target` _asx_base_luner_2)
      (`BlackboardComponent.SetValueAsString` (`AIBlueprintHelperLibrary.GetBlackboard` (`self.AICtrl`)) "cmd" "mine"))))

(event `on_cmd_stop`
  ;[1 1 1] cmd stop
  (`BlackboardComponent.SetValueAsString` (`AIBlueprintHelperLibrary.GetBlackboard` (`self.AICtrl`)) "cmd" "stop"))

(event `on_cmd_move`
  (params (move_to_point :type "Vector Structure"))
  ;[1 1 1] on cmd move
  (`BlackboardComponent.SetValueAsString` (`AIBlueprintHelperLibrary.GetBlackboard` (`self.AICtrl`)) "cmd" "stop")
  (`BlackboardComponent.SetValueAsVector` (`AIBlueprintHelperLibrary.GetBlackboard` (`self.AICtrl`)) "move_to_point" move_to_point)
  (`self.on_cmd_action` "move")
  (`BlackboardComponent.SetValueAsString` (`AIBlueprintHelperLibrary.GetBlackboard` (`self.AICtrl`)) "cmd" "move"))

(fn `UserConstructionScript`)