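; Test ship built on an XCore action and flight system that flies between three target actors.
; BeginPlay initializes it, sets its flight tuning in FlyData, then follows Target1 after a short delay.
; Each completed XAction triggers a MoveToLocation to the target selected by TargetNum, which cycles through the three in a loop.
; Goto randomly shifts Target1 and moves to it, but its only caller is unwired, alongside other leftover debug chains.
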(event `self.ReceiveBeginPlay`
  (bind _flydata (`self.flyData`))
  (`parent.ReceiveBeginPlay`)
  (add `self.onXActionDone` (delegate `onXActionDone_Event_1`))
  (`self.Init`)
  (set `FlyData.brakingPower` 3000.0 _flydata)
  (set `FlyData.accelerationPower` 400.0 _flydata)
  (set `FlyData.maxSpeed` 2000.0 _flydata)
  (set `FlyData.brakingDistances` 1000.0 _flydata)
  (set `FlyData.rotationPower` 5.0 _flydata)
  (set `FlyData.stopDistances` 100.0 _flydata)
  (`KismetSystemLibrary.Delay` 3.0)
  (`self.followActor` (`self.target1`)))

(event `onXActionDone_Event_1` :!signature `self.onXActionDone`
  (params (uXAction :type "XAction Object Reference"))
  (if (== (`self.targetNum`) 1)
    (`self.moveToLocation` (`self.K2_GetActorLocation` (`self.target1`)))
    (set `self.targetNum` 2)
    (elif (== (`self.targetNum`) 2)
      (`self.moveToLocation` (`self.K2_GetActorLocation` (`self.target2`)))
      (set `self.targetNum` 3)
      (elif (== (`self.targetNum`) 3)
        (`self.moveToLocation` (`self.K2_GetActorLocation` (`self.target3`)))
        (set `self.targetNum` 1)))))

(event `self.ReceiveTick`
  (params (DeltaSeconds :type "Float (single-precision)")))

(event `Goto`
  (`self.K2_SetActorLocation` (`self.target1`) (`KismetMathLibrary.MakeVector` (+ (.x (`self.K2_GetActorLocation` (`self.target1`))) (`KismetMathLibrary.RandomFloatInRange` -2000.0 2000.0)) (+ (.y (`self.K2_GetActorLocation` (`self.target1`))) (`KismetMathLibrary.RandomFloatInRange` -2000.0 2000.0)) (.z (`self.K2_GetActorLocation` (`self.target1`)))) false false)
  (`self.moveToLocation` (`self.K2_GetActorLocation` (`self.target1`))))

(fn `UserConstructionScript`)