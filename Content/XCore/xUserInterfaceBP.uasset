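; Player pawn for the space game that hosts the object overview UI and follows a selected SpaceObject.
; On BeginPlay it possesses itself, shows the cursor, creates and updates the W_spaceObjectList widget, and binds to xspaceGameMode follow/unfollow events.
; Following snaps it above the target at a fixed height offset, then Tick matches the target's X/Y while keeping its own Z until unfollowed.
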(event `self.ReceiveBeginPlay`
  (bind _returnvalue (`GameplayStatics.GetPlayerController` 0))
  (set `PlayerController.bShowMouseCursor` true _returnvalue)
  (`Controller.Possess` _returnvalue self)
  (bind _asxspace_game_mode (cast `xspaceGameMode` (`GameplayStatics.GetGameMode`)))
  (bind _output_get (set `self.gameMode_0` _asxspace_game_mode))
  (add `xspaceGameMode.onFollowTarget_listWiget` _output_get (delegate `onFollowTarget_listWiget_Event_0`))
  (add `xspaceGameMode.onUnFollowTarget_listWiget` (`self.gameMode_0`) (delegate `onUnFollowTarget_listWiget_Event_0`))
  (`self.CreateOverview`))

(event `onUnFollowTarget_listWiget_Event_0`
  (set `self.followTarget` null))

(event `onFollowTarget_listWiget_Event_0`
  (params (spaceObject :type "Actor Object Reference"))
  (bind _asspace_object (cast `SpaceObject` spaceObject))
  (bind _output_get (set `self.followTarget` _asspace_object))
  (`self.onSetFollowTarget` _output_get))

(event `self.ReceiveTick`
  (params (DeltaSeconds :type "Float (single-precision)"))
  (`parent.ReceiveTick` DeltaSeconds)
  (`self.onFollowSpaceObject` 0.0))

(event `CreateOverview`
  ;[0.8632 1 0.7379] Create overview
  (bind _returnvalue (`|CreateWidget` "/Game/XCore/UI/W_spaceObjectList.W_spaceObjectList_C" (`GameplayStatics.GetPlayerController` 0)))
  (bind _output_get (set `self.w_overview` _returnvalue))
  (`UserWidget.AddToViewport` _output_get 0)
  (`self.UpdateOverview`))

(event `UpdateOverview`
  ;[0.8632 1 0.7379] Update overview
  (`/Game/XCore/UI/W_spaceObjectList.onUpdate_Event` (`self.w_overview`)))

(event `onFollowSpaceObject`
  (params (DeltaTime :type "Float (double-precision)"))
  ;[0.8076 0.7299 1] onFollowSpaceObject
  (if (`KismetSystemLibrary.IsValid` (`self.followTarget`))
    (`self.K2_SetActorLocation` (`KismetMathLibrary.MakeVector` (.x (`self.K2_GetActorLocation` (`self.followTarget`))) (.y (`self.K2_GetActorLocation` (`self.followTarget`))) (.z (`self.K2_GetActorLocation`))))))

(event `onSetFollowTarget`
  (params (spaceObject :type "SpaceObject Object Reference"))
  ;[1 1 1] onSetFollowTarget
  (set `self.followTarget` spaceObject)
  (`self.K2_SetActorLocation` (`KismetMathLibrary.MakeVector` (.x (`self.K2_GetActorLocation` (`self.followTarget`))) (.y (`self.K2_GetActorLocation` (`self.followTarget`))) (+ (.z (`self.K2_GetActorLocation` (`self.followTarget`))) 900.0))))

(fn `UserConstructionScript`)